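; Pushable puzzle prop that the player shoves along world -Y from a fixed camera, with inner/outer interaction icons shown while the Monocle is active.
; Interacting inside the inner sphere fades the screen, snaps the player to StartArrow and switches to the prop's camera.
; Holding W makes Tick move mesh, camera and player together.
; When the player leaves EndBoxCollision, control returns and a static BP_DeadObject replaces the prop.
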(event `self.ReceiveTick`
  (params (DeltaSeconds :type "Float (single-precision)"))
  (bind _returnvalue (* DeltaSeconds -100.0))
  (bind _camera (`self.Camera`))
  (bind _staticmesh (`self.StaticMesh`))
  (bind (_returnvalue_x _returnvalue_y _returnvalue_z) (`KismetMathLibrary.BreakVector` (`SceneComponent.K2_GetComponentLocation` _camera)))
  (bind (_returnvalue_x_2 _returnvalue_y_2 _returnvalue_z_2) (`KismetMathLibrary.BreakVector` (`SceneComponent.K2_GetComponentLocation` _staticmesh)))
  (bind _rootcomponent (`Actor.RootComponent` (`self.FirstPersonRef`)))
  (bind (_returnvalue_x_3 _returnvalue_y_3 _returnvalue_z_3) (`KismetMathLibrary.BreakVector` (`SceneComponent.K2_GetComponentLocation` _rootcomponent)))
  (if (`/Game/FirstPerson/Blueprints/BP_FirstPersonCharacter.InPush?` (`self.FirstPersonRef`))
    ;[1 1 1] Move Pushable Item
    (if (`self.InCam?`)
      (if (`PlayerController.IsInputKeyDown` (`GameplayStatics.GetPlayerController` 0) "W")
        (`SceneComponent.K2_SetWorldLocation` _camera (`KismetMathLibrary.MakeVector` _returnvalue_x (+ _returnvalue_y _returnvalue) _returnvalue_z) false false)
        (`SceneComponent.K2_SetWorldLocation` _staticmesh (`KismetMathLibrary.MakeVector` _returnvalue_x_2 (+ _returnvalue_y_2 _returnvalue) _returnvalue_z_2) false false)
        (`SceneComponent.K2_SetWorldLocation` _rootcomponent (`KismetMathLibrary.MakeVector` _returnvalue_x_3 (+ _returnvalue_y_3 _returnvalue) _returnvalue_z_3) false false)))
    (else
      ;[1 1 1] Is Monocle Activated?
      (bind _asbp_first_person_character (cast `/Game/FirstPerson/Blueprints/BP_FirstPersonCharacter` (`GameplayStatics.GetPlayerCharacter` 0)))
      (if (`/Game/FirstPerson/Blueprints/BP_FirstPersonCharacter.Monocle?` _asbp_first_person_character)
        (if (`PrimitiveComponent.IsOverlappingActor` (`self.InnerSphereCollision`) _asbp_first_person_character)
          ;[1 1 1] Show Inner, Hide Outer
          (`SceneComponent.SetVisibility` (`self.InnerInteractionIcon`) true false)
          (`SceneComponent.SetVisibility` (`self.OuterInteractionIcon`) false false)
          (else
            ;[1 1 1] Show Outer, Hide Inner
            (if (`PrimitiveComponent.IsOverlappingActor` (`self.OuterSphereCollision`) _asbp_first_person_character)
              (`SceneComponent.SetVisibility` (`self.OuterInteractionIcon`) true false)
              (`SceneComponent.SetVisibility` (`self.InnerInteractionIcon`) false false))))
        (else
          ;[1 1 1] Show No Icon When Monocle is not active
          (`SceneComponent.SetVisibility` (`self.InnerInteractionIcon`) false false)
          (`SceneComponent.SetVisibility` (`self.OuterInteractionIcon`) false false))))))

(event `CameraFade`
  (params (CameraManager :type "PlayerCameraManager Object Reference") (StartFadeTime :type "Float (double-precision)") (DurationBetween :type "Float (double-precision)") (EndFadeTime :type "Float (double-precision)"))
  (`PlayerCameraManager.StartCameraFade` :`self` CameraManager :`ToAlpha` 1.0 :`Duration` StartFadeTime)
  (`KismetSystemLibrary.Delay` DurationBetween)
  (`PlayerCameraManager.StartCameraFade` :`self` CameraManager :`FromAlpha` 1.0 :`ToAlpha` 0.0 :`Duration` EndFadeTime))

(event `self.ReceiveBeginPlay`
  (bind _asbp_first_person_character (cast `/Game/FirstPerson/Blueprints/BP_FirstPersonCharacter` (`GameplayStatics.GetPlayerCharacter` 0)))
  (set `self.FirstPersonRef` _asbp_first_person_character))

(event `/Game/FirstPerson/Interfaces/InterfaceInteract.InteractFunction`
  (params (Character :type "/Game/FirstPerson/Blueprints/BP_FirstPersonCharacter Object Reference"))
  (bind _firstpersonref (`self.FirstPersonRef`))
  (bind (_returnvalue_location _returnvalue_rotation) (`KismetMathLibrary.BreakTransform` (`SceneComponent.K2_GetComponentToWorld` (`self.StartArrow`))))
  (bind _charactermovement (`Character.CharacterMovement` (`self.FirstPersonRef`)))
  ;[1 1 1] Interact with Pushable
  (set `/Game/FirstPerson/Blueprints/BP_FirstPersonCharacter.PushForwardPuzzle` false _firstpersonref)
  (if (`PrimitiveComponent.IsOverlappingActor` (`self.InnerSphereCollision`) (`GameplayStatics.GetPlayerCharacter` 0))
    (`ActorComponent.Activate` (`self.Camera`) false)
    (`CharacterMovementComponent.DisableMovement` (`Character.CharacterMovement` _firstpersonref))
    (`Controller.SetIgnoreLookInput` (`GameplayStatics.GetPlayerController` 0) true)
    (`self.CameraFade` (`GameplayStatics.GetPlayerCameraManager` 0) 0.25 0.5 0.25)
    (`KismetSystemLibrary.Delay` 0.5)
    (set `/Game/FirstPerson/Blueprints/BP_FirstPersonCharacter.InPush?` true (`self.FirstPersonRef`))
    (`SceneComponent.K2_SetWorldTransform` (`Actor.RootComponent` (`GameplayStatics.GetPlayerCharacter` 0)) (`KismetMathLibrary.MakeTransform` _returnvalue_location _returnvalue_rotation) false false)
    (`Controller.SetControlRotation` (`GameplayStatics.GetPlayerController` 0) (`self.K2_GetActorRotation` (`GameplayStatics.GetPlayerCharacter` 0)))
    (set `self.InCam?` true)
    (`PlayerController.SetViewTargetWithBlend` (`GameplayStatics.GetPlayerController` 0) (`ActorComponent.GetOwner` (`self.Camera`)) 0.0 "VTBlend_Linear" 0.0 false)
    (`SkeletalMeshComponent.SetAnimationMode` (`Character.Mesh` (`GameplayStatics.GetPlayerCharacter` 0)) "AnimationSingleNode" true)
    (`CharacterMovementComponent.SetMovementMode` _charactermovement (`CharacterMovementComponent.DefaultLandMovementMode` _charactermovement) 0)))

(event `self.EndBoxCollision.OnComponentEndOverlap`
  (params (OverlappedComponent :type "PrimitiveComponent Object Reference") (OtherActor :type "Actor Object Reference") (OtherComp :type "PrimitiveComponent Object Reference") (OtherBodyIndex :type Integer))
  (bind _firstpersonref (`self.FirstPersonRef`))
  (bind (_returnvalue_location _returnvalue_rotation) (`KismetMathLibrary.BreakTransform` (`SceneComponent.K2_GetComponentToWorld` (`self.StaticMesh`))))
  (bind _charactermovement (`Character.CharacterMovement` _firstpersonref))
  ;[1 1 1] End Interact with Pushable
  (if (and (== OtherActor (`GameplayStatics.GetPlayerCharacter` 0)) (`self.InCam?`))
    (`self.CameraFade` (`GameplayStatics.GetPlayerCameraManager` 0) 0.1 0.25 0.1)
    (`KismetSystemLibrary.Delay` 0.25)
    (set `/Game/FirstPerson/Blueprints/BP_FirstPersonCharacter.InPush?` false (`self.FirstPersonRef`))
    (`Controller.ResetIgnoreLookInput` (`GameplayStatics.GetPlayerController` 0))
    (`SkeletalMeshComponent.SetAnimationMode` (`Character.Mesh` (`GameplayStatics.GetPlayerCharacter` 0)) "AnimationBlueprint" true)
    (`CharacterMovementComponent.SetMovementMode` _charactermovement (`CharacterMovementComponent.DefaultLandMovementMode` _charactermovement) 0)
    (set `self.InCam?` false)
    (`ActorComponent.Deactivate` (`self.Camera`))
    (`PlayerController.SetViewTargetWithBlend` (`GameplayStatics.GetPlayerController` 0) _firstpersonref 0.0 "VTBlend_Linear" 0.0 false)
    (bind _returnvalue (`|SpawnActorFromClass` "/Game/Props/Pushable/BP_DeadObject.BP_DeadObject_C" (`KismetMathLibrary.MakeTransform` (+ _returnvalue_location (5.0 0.0 0.0)) _returnvalue_rotation (`self.ObjectScale`)) "Undefined" "MultiplyWithRoot" null null))
    (`StaticMeshComponent.SetStaticMesh` (`/Game/Props/Pushable/BP_DeadObject.PushedObject` _returnvalue) (`self.ObjectMesh`))
    (`KismetSystemLibrary.Delay` 0.2)
    (`self.K2_DestroyActor`)))

(fn `UserConstructionScript`
  (bind _endboxcollision (`self.EndBoxCollision`))
  (bind _camera (`self.Camera`))
  (bind _startarrow (`self.StartArrow`))
  (`|ExecutionSequence`
    (:`then_0`
      (if (`self.Debugging?`)
        (`SceneComponent.SetHiddenInGame` (`self.StartBoxCollision`) false false)
        (`SceneComponent.SetHiddenInGame` (`self.EndBoxCollision`) false false)))
    (:`then_1`
      (`SceneComponent.K2_SetWorldLocation` _startarrow (+ (`SceneComponent.K2_GetComponentLocation` _startarrow) (`self.CharacterOffsetLocation`)) false false))
    (:`then_2`
      (`SceneComponent.K2_SetRelativeLocation` _camera (`SceneComponent.RelativeLocation` _camera) false false))
    (:`then_3`
      (`SceneComponent.SetWorldScale3D` (`self.StaticMesh`) (`self.ObjectScale`))
      (`StaticMeshComponent.SetStaticMesh` (`self.StaticMesh`) (`self.ObjectMesh`)))
    (:`then_4`
      (`SceneComponent.K2_SetWorldLocation` _endboxcollision (+ (`SceneComponent.K2_GetComponentLocation` _endboxcollision) (`self.EndOffsetLocation`)) false false))))