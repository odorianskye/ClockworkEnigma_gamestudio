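; Player controller component that drives a fade-in/fade-out post-process scan effect through StartScan and EndScan.
; A five-state machine advances a normalized time on tick, switching tick off when faded out or invalid.
; MPC_Scan receives time, state flags, grid settings and pawn location.
; A lazily spawned BP_Scan_Actor carries the dynamic post-process material, with blend weight shaped by an optional curve.
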(event `self.ReceiveBeginPlay`
  (bind _asplayer_controller (cast `PlayerController` (`self.GetOwner`))
    (:`then`
      (set `self.PlayerController` _asplayer_controller)
      (`self.UpdateScanState` "NewEnumerator3" true)
      (`KismetMaterialLibrary.SetScalarParameterValue` "/Game/CE_GrayBox/Scan/Materials/ParameterCollections/MPC_Scan.MPC_Scan" "Range" (`self.GridCellSize`))
      (`KismetMaterialLibrary.SetScalarParameterValue` "/Game/CE_GrayBox/Scan/Materials/ParameterCollections/MPC_Scan.MPC_Scan" "GridCellSize" (`self.Range`)))
    (:`CastFailed`
      (`self.UpdateScanState` "NewEnumerator4" true))))

(event `self.ReceiveTick`
  (params (DeltaSeconds :type "Float (single-precision)"))
  (bind _playercontroller (`self.PlayerController`))
  (bind _returnvalue (`Controller.K2_GetPawn` _playercontroller))
  (`self.UpdateScanTime` DeltaSeconds)
  (`KismetSystemLibrary.PrintString` (`KismetStringLibrary.Conv_DoubleToString` (`self.ScanNormalizedTime`)) true false (struct :`G` 0.66 :`B` 1.0 :`A` 1.0) 0.0)
  (`KismetSystemLibrary.PrintString` (`|GetEnumeratorNameAsString` (`self.State`)) true false (struct :`G` 0.66 :`B` 1.0 :`A` 1.0) 0.0)
  (switch `/Game/CE_GrayBox/Scan/_Enums/EBP_Scan_State` (`self.GetScanState`)
    (:`NewEnumerator0`
      (`self.UpdateScanPPBlendWeight` :!label _label))
    (:`NewEnumerator1`
      _)
    (:`NewEnumerator2`
      (goto _label))
    (:`NewEnumerator3`
      _))
  (`/Engine/EditorBlueprintResources/StandardMacros.IsValid` _playercontroller
    (:`Is Valid`
      (`/Engine/EditorBlueprintResources/StandardMacros.IsValid` _returnvalue
        (:`Is Valid`
          (`KismetMaterialLibrary.SetVectorParameterValue` "/Game/CE_GrayBox/Scan/Materials/ParameterCollections/MPC_Scan.MPC_Scan" "Location" (`KismetMathLibrary.Conv_VectorToLinearColor` (`Actor.K2_GetActorLocation` _returnvalue))))))))

(fn `DestroyPPActor`
  (bind _scan_actor (`self.Scan Actor`))
  (if (and (`KismetSystemLibrary.IsValid` _scan_actor) (`self.bDestroyActor`))
    (`Actor.K2_DestroyActor` _scan_actor)
    (set `self.Scan Actor` null)))

(fn `End Scan`
  (returns (bEnded :type Boolean))
  (switch `/Game/CE_GrayBox/Scan/_Enums/EBP_Scan_State` (`self.GetScanState`)
    (:`NewEnumerator0`
      _)
    (:`NewEnumerator1`
      _)
    (:`NewEnumerator2`
      (return false))
    (:`NewEnumerator3`
      (return false))
    (:`NewEnumerator4`
      (return false)))
  (bind _bupdated (`self.UpdateScanState` "NewEnumerator2"))
  (return _bupdated))

(fn `GetScanPPActor`
  (returns (ScanActor :type "/Game/CE_GrayBox/Scan/Blueprints/BP_Scan_Actor Object Reference"))
  (bind _scan_actor (`self.Scan Actor`))
  (bind _ppmaterial (`self.PPMaterial`))
  (bind _postprocess (`/Game/CE_GrayBox/Scan/Blueprints/BP_Scan_Actor.PostProcess` (`self.Scan Actor`)))
  (`/Engine/EditorBlueprintResources/StandardMacros.IsValid` _scan_actor
    (:`Is Valid`
      (return _scan_actor))
    (:`Is Not Valid`
      (bind _returnvalue (`|SpawnActorFromClass` "/Game/CE_GrayBox/Scan/Blueprints/BP_Scan_Actor.BP_Scan_Actor_C" (`KismetMathLibrary.MakeTransform` (0.0 0.0 0.0)) "Undefined" "MultiplyWithRoot" null null))
      (set `self.Scan Actor` _returnvalue)
      (`|ExecutionSequence`
        (:`then_0`
          (`/Engine/EditorBlueprintResources/StandardMacros.IsValid` (`self.PPMID`)
            (:`Is Valid`
              _)
            (:`Is Not Valid`
              (`/Engine/EditorBlueprintResources/StandardMacros.IsValid` _ppmaterial
                (:`Is Valid`
                  (bind _returnvalue_2 (`KismetMaterialLibrary.CreateDynamicMaterialInstance` _ppmaterial))
                  (set `self.PPMID` _returnvalue_2)))))
          (`/Engine/EditorBlueprintResources/StandardMacros.IsValid` _postprocess
            (:`Is Valid`
              (setmembers `PostProcessSettings` :`StructRef` (`PostProcessComponent.Settings` _postprocess) :`WeightedBlendables` (make `WeightedBlendables` (`|MakeArray` (make `WeightedBlendable` 1.0 (`self.PPMID`))))))))
        (:`then_1`
          (return _scan_actor))))))

(fn `GetScanState`
  (returns (State :type "/Game/CE_GrayBox/Scan/_Enums/EBP_Scan_State Enum"))
  (return (`self.State`)))

(fn `Start Scan`
  (returns (bStarted :type Boolean))
  (switch `/Game/CE_GrayBox/Scan/_Enums/EBP_Scan_State` (`self.GetScanState`)
    (:`NewEnumerator0`
      _)
    (:`NewEnumerator1`
      _)
    (:`NewEnumerator2`
      (bind _bupdated (`self.UpdateScanState` "NewEnumerator0" :!label _label))
      (return _bupdated))
    (:`NewEnumerator3`
      (goto _label))
    (:`NewEnumerator4`
      _))
  (return false))

(fn `UpdateScanPPBlendWeight`
  (locals (ThisTime :type "Float (single-precision)" :default 0.0))
  (bind _ppblendcurve (`self.PPBlendCurve`))
  (bind _scannormalizedtime (`self.ScanNormalizedTime`))
  (`/Engine/EditorBlueprintResources/StandardMacros.IsValid` _ppblendcurve
    (:`Is Valid`
      (set `local.ThisTime` (`CurveFloat.GetFloatValue` _ppblendcurve _scannormalizedtime)))
    (:`Is Not Valid`
      (set `local.ThisTime` _scannormalizedtime)))
  (bind _scanactor (`self.GetScanPPActor`))
  (`/Engine/EditorBlueprintResources/StandardMacros.IsValid` _scanactor
    (:`Is Valid`
      (bind _postprocess (`/Game/CE_GrayBox/Scan/Blueprints/BP_Scan_Actor.PostProcess` _scanactor))
      (`/Engine/EditorBlueprintResources/StandardMacros.IsValid` _postprocess
        (:`Is Valid`
          (set `PostProcessComponent.BlendWeight` (`local.ThisTime`) _postprocess))))))

(fn `UpdateScanState`
  (params (State :type "/Game/CE_GrayBox/Scan/_Enums/EBP_Scan_State Enum" :default "NewEnumerator0") (bForce :type Boolean))
  (returns (bUpdated :type Boolean))
  (if (or (`|EnumInequality` State (`self.State`)) bForce)
    (`|ExecutionSequence`
      (:`then_0`
        (switch `/Game/CE_GrayBox/Scan/_Enums/EBP_Scan_State` (`self.State`) ; exit current state
          (:`NewEnumerator1`
            (`KismetMaterialLibrary.SetScalarParameterValue` "/Game/CE_GrayBox/Scan/Materials/ParameterCollections/MPC_Scan.MPC_Scan" "bIsFadedIn"))
          (:`NewEnumerator3`
            (`KismetMaterialLibrary.SetScalarParameterValue` "/Game/CE_GrayBox/Scan/Materials/ParameterCollections/MPC_Scan.MPC_Scan" "bIsFadedOut")
            (`self.SetComponentTickEnabled` true))))
      (:`then_1`
        (bind _output_get (set `self.State` State))
        (switch `/Game/CE_GrayBox/Scan/_Enums/EBP_Scan_State` _output_get ; enter new state
          (:`NewEnumerator1`
            (`KismetMaterialLibrary.SetScalarParameterValue` "/Game/CE_GrayBox/Scan/Materials/ParameterCollections/MPC_Scan.MPC_Scan" "bIsFadedIn" 1.0)
            (`self.UpdateScanPPBlendWeight`))
          (:`NewEnumerator3`
            (`KismetMaterialLibrary.SetScalarParameterValue` "/Game/CE_GrayBox/Scan/Materials/ParameterCollections/MPC_Scan.MPC_Scan" "bIsFadedOut" 1.0)
            (`self.UpdateScanPPBlendWeight`)
            (`self.SetComponentTickEnabled` false :!label _label)
            (`self.DestroyPPActor`))
          (:`NewEnumerator4`
            (goto _label))))
      (:`then_2`
        (return true)))
    (else
      (return false))))

(fn `UpdateScanTime`
  (params (DeltaTime :type "Float (double-precision)"))
  (returns (bUpdated :type Boolean))
  (`|ExecutionSequence`
    (:`then_0`
      (switch `/Game/CE_GrayBox/Scan/_Enums/EBP_Scan_State` (`self.GetScanState`)
        (:`NewEnumerator0`
          (bind _output_get (set `self.ScanNormalizedTime` (+ (`self.ScanNormalizedTime`) (* (`local.DeltaTime`) (`self.FadeInSpeed`)))))
          (if (>= _output_get 1.0)
            (bind _output_get_2 (set `self.ScanNormalizedTime` 1.0))
            (`|ExecutionSequence`
              (:`then_0`
                (`KismetMaterialLibrary.SetScalarParameterValue` "/Game/CE_GrayBox/Scan/Materials/ParameterCollections/MPC_Scan.MPC_Scan" "NormalizedTime" _output_get_2 :!label _label))
              (:`then_1`
                (`self.UpdateScanState` "NewEnumerator1")))))
        (:`NewEnumerator2`
          (bind _output_get_3 (set `self.ScanNormalizedTime` (- (`self.ScanNormalizedTime`) (* (`local.DeltaTime`) (`self.FadeOutSpeed`))) :!label _label_2))
          (if (<= _output_get_3 0.0)
            (set `self.ScanNormalizedTime` 0.0)
            (`|ExecutionSequence`
              (:`then_0`
                (goto _label))
              (:`then_1`
                (`self.UpdateScanState` "NewEnumerator3")))
            (else
              (goto _label))))
        (:`NewEnumerator3`
          (goto _label_2))
        (:`NewEnumerator4`
          (return false))))
    (:`then_1`
      (return true))))