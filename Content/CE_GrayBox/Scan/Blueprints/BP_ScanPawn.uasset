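; BP_ScanPawn is a gray-box pawn that turns the IA_Scan input action into scan start and stop requests.
; On input start and completion it looks up BP_Scan_ControllerComponent on its controller and calls StartScan or EndScan, with validity checks and debug prints.
; The scan logic lives in that controller component; the pawn only forwards input.
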(event `EnhancedInput|/Game/CE_GrayBox/Scan/Inputs/IA_Scan`
  (params (ActionValue :type Boolean) (ElapsedSeconds :type "Float (double-precision)") (TriggeredSeconds :type "Float (double-precision)") (InputAction :type "InputAction Object Reference" :default "/Game/CE_GrayBox/Scan/Inputs/IA_Scan.IA_Scan"))
  (bind _returnvalue (`self.GetController`))
  (bind _returnvalue_2 (`self.GetController`))
  (bind _returnvalue_3 (`self.GetComponentByClass` _returnvalue_2 "/Game/CE_GrayBox/Scan/Blueprints/BP_Scan_ControllerComponent.BP_Scan_ControllerComponent_C"))
  (bind _returnvalue_4 (`self.GetComponentByClass` _returnvalue "/Game/CE_GrayBox/Scan/Blueprints/BP_Scan_ControllerComponent.BP_Scan_ControllerComponent_C"))
  (:`Started`
    (`/Engine/EditorBlueprintResources/StandardMacros.IsValid` _returnvalue
      (:`Is Valid`
        (`/Engine/EditorBlueprintResources/StandardMacros.IsValid` _returnvalue_4
          (:`Is Valid`
            (`/Game/CE_GrayBox/Scan/Blueprints/BP_Scan_ControllerComponent.Start Scan` _returnvalue_4)
            (`KismetSystemLibrary.PrintString` "Start Scan"))))))
  (:`Completed`
    (`/Engine/EditorBlueprintResources/StandardMacros.IsValid` _returnvalue_2
      (:`Is Valid`
        (`/Engine/EditorBlueprintResources/StandardMacros.IsValid` _returnvalue_3
          (:`Is Valid`
            (`/Game/CE_GrayBox/Scan/Blueprints/BP_Scan_ControllerComponent.End Scan` _returnvalue_3)
            (`KismetSystemLibrary.PrintString` "End Scan")))))))

(fn `UserConstructionScript`)